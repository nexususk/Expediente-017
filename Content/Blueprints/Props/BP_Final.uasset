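; BP_Final is the end-of-game trigger prop that fires when the first-person character overlaps its box.
; It stops the character's timer, plays a 2D sound and fades the camera to white.
; After the fade it shows a WBP_LevelVideo widget with the chosen video.
; When the media player reports the end of playback, it opens the main menu level.
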(event `self.Box.OnComponentBeginOverlap`
  (params (OverlappedComponent :type "PrimitiveComponent Object Reference") (OtherActor :type "Actor Object Reference") (OtherComp :type "PrimitiveComponent Object Reference") (OtherBodyIndex :type Integer) (bFromSweep :type Boolean) (SweepResult :type "HitResult Structure (by ref)"))
  (bind _asbp_first_person_character (cast `/Game/FirstPerson/Blueprints/BP_FirstPersonCharacter` OtherActor))
  (set `/Game/FirstPerson/Blueprints/BP_FirstPersonCharacter.TemporizadorActivo?` false _asbp_first_person_character)
  (`GameplayStatics.PlaySound2D` null 1.0 1.0 0.0 null null)
  (`PlayerCameraManager.StartCameraFade` (`GameplayStatics.GetPlayerCameraManager` 0) 0.0 1.0 1.5 (struct :`R` 1.0 :`G` 1.0 :`B` 1.0 :`A` 1.0) false true)
  (`KismetSystemLibrary.Delay` 1.5)
  (bind _returnvalue (`|CreateWidget` "/Game/UI/WBP_LevelVideo.WBP_LevelVideo_C" null "/Game/Media/videoplayback.videoplayback"))
  (`UserWidget.AddToViewport` _returnvalue 0)
  (add `MediaPlayer.OnEndReached` (`self.ReproductorVideo`) (delegate `VideoEnd`)))

(event `VideoEnd`
  (`GameplayStatics.OpenLevelBySoftObjectPtr` "/Game/Levels/MenuPpal.MenuPpal"))

(fn `UserConstructionScript`)