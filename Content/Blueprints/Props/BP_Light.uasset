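; BP_Light is a light prop that ends the game when the player stays exposed to it.
; Each tick it line-traces on the Visibility channel from its PointLight to the player character, with no range check.
; Unbroken line of sight accumulates a timer, which resets when the trace fails to hit the player.
; After half a second it shows the WBP_MenuMuerte death menu, switches to UI-only input and pauses.
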(event `self.ReceiveTick`
  (params (DeltaSeconds :type "Float (single-precision)"))
  (bind _returnvalue (`GameplayStatics.GetPlayerController` 0))
  (bind _timeinlight (`self.TimeInLight`))
  (bind _outhit (`KismetSystemLibrary.LineTraceSingle` (`SceneComponent.K2_GetComponentLocation` (`self.PointLight`)) (`self.K2_GetActorLocation` (`GameplayStatics.GetPlayerCharacter` 0)) "TraceTypeQuery1"))
  (if (== (`.HitActor` (`GameplayStatics.BreakHitResult` _outhit)) (`GameplayStatics.GetPlayerCharacter` 0))
    (set `self.TimeInLight` (+ _timeinlight DeltaSeconds))
    (if (>= _timeinlight 0.5)
      (`KismetSystemLibrary.PrintString` "Golpeando")
      (bind _returnvalue_2 (`|CreateWidget` "/Game/Widgets/MenuMuerte/WBP_MenuMuerte.WBP_MenuMuerte_C"))
      (`UserWidget.AddToViewport` _returnvalue_2 0)
      (set `PlayerController.bShowMouseCursor` true _returnvalue)
      (`WidgetBlueprintLibrary.SetInputMode_UIOnlyEx` _returnvalue null)
      (`GameplayStatics.SetGamePaused` true))
    (else
      (set `self.TimeInLight` 0.0))))

(fn `UserConstructionScript`)